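; BP_Earth is the Earth actor, which holds BP_Country child actors and reports which countries are valid for a given region index.
; GetValidCountries looks up each child's country enum in DT_Countries and collects unique rows whose region number is at or below the index.
; An index at or above a hardcoded threshold includes every country found, and missing table rows are reported with a printed message.
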(fn `GetValidCountries`
  (params (RegionIndex :type Integer))
  (returns (ValidCountries :type "Array of /Game/SCountryData Structure"))
  (locals (ValidCountries :type "Array of /Game/SCountryData Structure"))
  (for _array_element (`self.GetAllChildActors` true)
    (bind _asbp_country (cast `/Game/Earth/BP_Country` _array_element))
    (bind _returnvalue (`KismetStringLibrary.Conv_StringToName` (`|GetEnumeratorNameAsString` (`/Game/Earth/BP_Country.Country` _asbp_country))))
    (bind _returnvalue_2 (`|GetDataTableRow` "/Game/DT_Countries.DT_Countries" _returnvalue)
      (:`then`
        (if (>= RegionIndex 8)
          (`KismetArrayLibrary.Array_AddUnique` (`local.ValidCountries`) _returnvalue_2)
          (elif (<= (`.RegionNo_8_D8E055C34FBFA080828DD8B04F07D255` (break `/Game/SCountryData` _returnvalue_2)) RegionIndex)
            (`KismetArrayLibrary.Array_AddUnique` (`local.ValidCountries`) _returnvalue_2))))
      (:`RowNotFound`
        (`KismetSystemLibrary.PrintText` (`|FormatText` "{1} not found" _returnvalue)))))
  (return (`local.ValidCountries`)))

(fn `UserConstructionScript`)