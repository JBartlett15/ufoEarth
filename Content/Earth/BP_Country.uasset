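; BP_Country is an Earth map actor representing a single country chosen by its Country enum.
; Its Construction Script looks up the enum name in DT_Countries, then sets the row's mesh, applies land and outline materials to slots 0 and 1, and stores the region number.
; A missing row prints a not-found warning, and the event graph holds no active logic.
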(fn `UserConstructionScript`
  (bind _staticmesh (`self.StaticMesh`))
  (bind _returnvalue (`|GetEnumeratorNameAsString` (`self.Country`)))
  (bind _returnvalue_2 (`|GetDataTableRow` "/Game/DT_Countries.DT_Countries" (`KismetStringLibrary.Conv_StringToName` _returnvalue))
    (:`then`
      (bind (_country _mesh _regionno) (break `/Game/SCountryData` _returnvalue_2))
      (`StaticMeshComponent.SetStaticMesh` _staticmesh _mesh)
      (`PrimitiveComponent.SetMaterial` _staticmesh 0 "/Game/Materials/LandMaterial.LandMaterial")
      (`PrimitiveComponent.SetMaterial` _staticmesh 1 "/Game/Materials/OutlineMaterial.OutlineMaterial")
      (set `self.Region` _regionno))
    (:`RowNotFound`
      (`KismetSystemLibrary.PrintString` (`KismetTextLibrary.Conv_TextToString` (`|FormatText` "{1} not found" _returnvalue))))))